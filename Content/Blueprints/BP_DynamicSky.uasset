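; Dynamic sky actor that runs a looping 24-hour day/night cycle, also previewed through the construction script.
; Time drives sun/moon rotation and visibility, sky-sphere star and moon material parameters, and day/night preset values copied into variables.
; Tick calls TODManager's UpdateTODData every frame until shortly after dusk, as its threshold test lacks an absolute value.
; Cloud handling is empty, and rain and snow setters are never called here.
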(event Custom|OnDayNightAlternated
  (bind _outactors (Actor|GetAllActorsOfClass "/Script/WeatherX.TODManager"))
  (Class|TODManager|UpdateTODData (Utilities|Array|Get(acopy) _outactors)))

(event EventBeginPlay
  (01-BasicSettings|InitSkySphereMaterial)
  (Variables|01-BasicSettings|SetDynamicTimeOfDay (Variables|01-BasicSettings|GetTimeOfDay)))

(event Collision|EventActorBeginOverlap
  (params (OtherActor :type Actor%20Object%20Reference)))

(event EventTick
  (params (DeltaSeconds :type Float%20%28single-precision%29))
  (Variables|01-BasicSettings|SetDynamicTimeOfDay (+ (* DeltaSeconds (Variables|01-BasicSettings|GetTODSpeed)) (Variables|01-BasicSettings|GetDynamicTimeOfDay)))
  (Variables|01-BasicSettings|SetTimeOfDay (.Remainder (Math|Float|Division(WholeandRemainder) (Variables|01-BasicSettings|GetDynamicTimeOfDay) 24.0)))
  (01-BasicSettings|HandleDynamics)
  (if (or (<= (- (Variables|01-BasicSettings|GetTimeOfDay) (- (Variables|01-BasicSettings|GetDawnTime) 0.3)) 0.1) (<= (- (Variables|01-BasicSettings|GetTimeOfDay) (+ (Variables|01-BasicSettings|GetDuskTime) 0.3)) 0.1))
    (CallFunction|OnDayNightAlternated)))

(fn ConstructionScript
  (bind _is_dynmi_skysphere_valid (01-BasicSettings|InitSkySphereMaterial))
  (if _is_dynmi_skysphere_valid
    (Utilities|FlowControl|Sequence
      (:then_0
        (01-BasicSettings|HandleSunMoonRotation))
      (:then_1
        (01-BasicSettings|HandleVisibility))
      (:then_2
        (02-NightSettings|HandleNightSettings))
      (:then_3
        (03-CloudSettings|HandleCloudSettings)))))

(fn HandleSunMoonRotation
  ;[0.15 0.15 0.15 0.5] Sun rotation between dawn and dust
  (Transformation|SetWorldRotation (Variables|Default|GetSunDirectionalLight) (Math|Rotator|MakeRotator 0.0 (Math|Float|MapRangeUnclamped (Variables|01-BasicSettings|GetTimeOfDay) (Variables|01-BasicSettings|GetDawnTime) (Variables|01-BasicSettings|GetDuskTime) 0.0 -1.8e+02) (Variables|01-BasicSettings|GetSunMoonRotation)) false false)
  (if (Utilities|IsNightTime)
    (if (>= (Variables|01-BasicSettings|GetTimeOfDay) (+ (Variables|01-BasicSettings|GetDuskTime) 0.3))
      ;[0.15 0.15 0.15 0.5] Moon rotation after dusk
      (Transformation|SetWorldRotation (Variables|Default|GetMoonDirectionalLight) (Math|Rotator|MakeRotator 0.0 (Math|Float|MapRangeUnclamped (Variables|01-BasicSettings|GetTimeOfDay) (Variables|01-BasicSettings|GetDuskTime) 24.0 -1.8e+02 -9e+01) (Variables|01-BasicSettings|GetSunMoonRotation)) false false)
      (else
        ;[0.15 0.15 0.15 0.5] Moon rotation before dawn
        (Transformation|SetWorldRotation (Variables|Default|GetMoonDirectionalLight) (Math|Rotator|MakeRotator 0.0 (Math|Float|MapRangeUnclamped (Variables|01-BasicSettings|GetTimeOfDay) 0.0 (Variables|01-BasicSettings|GetDawnTime) -9e+01 0.0) (Variables|01-BasicSettings|GetSunMoonRotation)) false false)))
    (else
      (Transformation|SetWorldRotation (Variables|Default|GetMoonDirectionalLight) (Math|Rotator|MakeRotator 0.0 0.0 0.0) false false))))

(fn HandleVisibility
  (Rendering|SetVisibility (Variables|Default|GetSunDirectionalLight) (Utilities|IsDayTime) false)
  (Rendering|SetVisibility (Variables|Default|GetMoonDirectionalLight) (Utilities|IsNightTime) false))

(fn HandleNightSettings
  (bind _created_dynmi_skysphere (Variables|01-BasicSettings|GetCreated_DynMI_SkySphere))
  (if (Utilities|IsNightTime)
    (Utilities|FlowControl|Sequence
      (:then_0
        (Variables|04-WeatherSettings|SetCurrentTODPreset "/WeatherX/DataAssets/DA_SunnyNight.DA_SunnyNight")
        (05-TODActorSettings|ApplyTODActorSettings))
      (:then_1
        ;[0.15 0.15 0.15 0.5] Night time sky sphere
        (Rendering|Material|SetScalarParameterValue _created_dynmi_skysphere "IsStarsVisible" (Math|Float|SelectFloat 1.0 0.0 (Variables|02-NightSettings|GetShouldShowStars)) :!class /Script/Engine.MaterialInstanceDynamic)
        (Rendering|Material|SetScalarParameterValue _created_dynmi_skysphere "IsMoonVisible" (Math|Float|SelectFloat 1.0 0.0 (Variables|02-NightSettings|GetShouldShowMoon)) :!class /Script/Engine.MaterialInstanceDynamic)
        (Rendering|Material|SetScalarParameterValue (Variables|01-BasicSettings|GetCreated_DynMI_SkySphere) "TimeOfDay" (Variables|01-BasicSettings|GetTimeOfDay) :!class /Script/Engine.MaterialInstanceDynamic)
        (Rendering|Material|SetScalarParameterValue (Variables|01-BasicSettings|GetCreated_DynMI_SkySphere) "StarsStrength" (Math|Float|Lerp 1.5 0.0 (Utilities|DayNightBlendAlpha -0.3 1.5)) :!class /Script/Engine.MaterialInstanceDynamic)))
    (else
      ;[0.15 0.15 0.15 0.5] Day time sky atmosphere & sky sphere
      (Variables|04-WeatherSettings|SetCurrentTODPreset "/WeatherX/DataAssets/DA_SunnyDay.DA_SunnyDay")
      (05-TODActorSettings|ApplyTODActorSettings)
      (Rendering|Material|SetScalarParameterValue (Variables|01-BasicSettings|GetCreated_DynMI_SkySphere) "IsStarsVisible" 0.0 :!class /Script/Engine.MaterialInstanceDynamic)
      (Rendering|Material|SetScalarParameterValue (Variables|01-BasicSettings|GetCreated_DynMI_SkySphere) "IsMoonVisible" 0.0 :!class /Script/Engine.MaterialInstanceDynamic))))

(fn InitSkySphereMaterial
  (bind _returnvalue (Rendering|Material|CreateDynamicMaterialInstance (Variables|Default|GetSM_SkySphere) 0 "/WeatherX/Materials/Sky/MI_DynamicSkySphere.MI_DynamicSkySphere" "None" :!class /Script/Engine.PrimitiveComponent))
  (bind _output_get (Variables|01-BasicSettings|SetCreated_DynMI_SkySphere _returnvalue))
  (return (Utilities|IsValid _output_get)))

(fn HandleCloudSettings)

(fn HandleDynamics
  (Utilities|FlowControl|Sequence
    (:then_0
      (01-BasicSettings|HandleSunMoonRotation))
    (:then_1
      (01-BasicSettings|HandleVisibility))
    (:then_2
      (02-NightSettings|HandleNightSettings))
    (:then_3
      (03-CloudSettings|HandleCloudSettings))))

(fn ApplyTODActorSettings
  (bind _currenttodpreset (Variables|04-WeatherSettings|GetCurrentTODPreset))
  (bind _directionallightsettings (Variables|/WeatherX/DataAssets/BP_WeatherDataAssetBase.BP_WeatherDataAssetBase_C|GetDirectionalLightSettings _currenttodpreset))
  (bind _skyatmospheresettings (Variables|/WeatherX/DataAssets/BP_WeatherDataAssetBase.BP_WeatherDataAssetBase_C|GetSkyAtmosphereSettings _currenttodpreset))
  (bind _exponentialheightfogsettings (Variables|/WeatherX/DataAssets/BP_WeatherDataAssetBase.BP_WeatherDataAssetBase_C|GetExponentialHeightFogSettings _currenttodpreset))
  (Variables|05-TODActorSettings|SetDirLightIntensity (.dirlightintensity _directionallightsettings))
  (Variables|05-TODActorSettings|SetDirLightColor (.dirlightcolor _directionallightsettings))
  (Variables|05-TODActorSettings|SetDirLightSourceAngle (.dirlightsourceangle _directionallightsettings))
  (Variables|05-TODActorSettings|SetDirLightTemperature (.dirlighttemperature _directionallightsettings))
  (Variables|05-TODActorSettings|SetSkyLightIntensity (.skylightintensity (Variables|/WeatherX/DataAssets/BP_WeatherDataAssetBase.BP_WeatherDataAssetBase_C|GetSkyLightSettings _currenttodpreset)))
  (Variables|05-TODActorSettings|SetMultiScattering (.multiscattering _skyatmospheresettings))
  (Variables|05-TODActorSettings|SetRayleighScattering (.rayleighscattering _skyatmospheresettings))
  (Variables|05-TODActorSettings|SetMieScatteringScale (.miescatteringscale _skyatmospheresettings))
  (Variables|05-TODActorSettings|SetMieAbsorptionScale (.mieabsorptionscale _skyatmospheresettings))
  (Variables|05-TODActorSettings|SetMieAnisotropy (.mieanisotropy _skyatmospheresettings))
  (Variables|05-TODActorSettings|SetAerial%20PerspectiveViewDistanceScale 0.0)
  (Variables|05-TODActorSettings|SetEmissiveColor (.emissivecolor _exponentialheightfogsettings))
  (Variables|05-TODActorSettings|SetExtinctionScale (.extinctionscale _exponentialheightfogsettings)))