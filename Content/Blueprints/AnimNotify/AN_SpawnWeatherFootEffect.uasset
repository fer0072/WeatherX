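; Anim notify that spawns left or right Niagara foot effects where a character's foot lands in snowy weather.
; When ShouldDoLineTrace passes, it traces downward from the landing foot bone against WorldStatic objects, then checks the weather type.
; The effect is nudged along the foot's yaw, and takes that yaw in IDLE-named animations or the owner's rotation otherwise.
; A puddle-splash branch based on surface type exists but never runs.
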(fn ReceivedNotify
  (params (MeshComp :type Skeletal%20Mesh%20Component%20Object%20Reference) (Animation :type Anim%20Sequence%20Base%20Object%20Reference) (EventReference :type Anim%20Notify%20Event%20Reference%20Structure%20%28by%20ref%29))
  (bind _returnvalue (Components|GetOwner MeshComp))
  (bind _returnvalue_2 (Transformation|GetActorRotation _returnvalue))
  (LocalVariables|SetCurrentAnimation Animation)
  (bind _returnvalue_3 (Utilities|ShouldDoLineTrace))
  (if _returnvalue_3
    (switch Utilities|FlowControl|Switch|SwitchonE_FootType (Variables|None|GetCurrentLandingFoot)
      (:NewEnumerator0
        (LocalVariables|SetCurrentLandingBoneName "foot_l"))
      (:NewEnumerator1
        (LocalVariables|SetCurrentLandingBoneName "foot_r")))
    (bind _outhit (Collision|LineTraceForObjects (Transformation|GetSocketLocation MeshComp (LocalVariables|GetCurrentLandingBoneName)) (+ (Transformation|GetSocketLocation MeshComp (LocalVariables|GetCurrentLandingBoneName)) (* (* (Math|Vector|GetUpVector MeshComp) -1.0) 1e+02)) (Utilities|Array|MakeArray "ObjectTypeQuery1") false 0 "None"))
    (LocalVariables|SetCurrentSurfaceHitResult _outhit)
    (Utilities|GetCurrentWeatherType
      (:Snowy
        (Niagara|SpawnSystematLocation (select (Utilities|String|Contains (Utilities|String|ToString(Name) (LocalVariables|GetCurrentLandingBoneName)) "_l") "/WeatherX/Niagara/Footprints/NS_LeftFoot.NS_LeftFoot" "/WeatherX/Niagara/Footprints/NS_RightFoot.NS_RightFoot") (+ (.Location (Collision|BreakHitResult (LocalVariables|GetCurrentSurfaceHitResult))) (* (Math|Rotator|GetRotationXVector (Math|Rotator|CombineRotators (Math|Rotator|MakeRotator 0.0 0.0 (+ (.Yaw (Math|Rotator|BreakRotator (.Rotation (Math|Transform|BreakTransform (Transformation|GetSocketTransform MeshComp (LocalVariables|GetCurrentLandingBoneName) "RTS_Actor"))))) (Math|Float|SelectFloat 1.8e+02 -3e+01 (Utilities|String|Contains (Utilities|String|ToString(Name) (LocalVariables|GetCurrentLandingBoneName)) "_r")))) _returnvalue_2)) 5.0)) (Math|Rotator|SelectRotator (Math|Rotator|CombineRotators (Math|Rotator|MakeRotator 0.0 0.0 (+ (.Yaw (Math|Rotator|BreakRotator (.Rotation (Math|Transform|BreakTransform (Transformation|GetSocketTransform MeshComp (LocalVariables|GetCurrentLandingBoneName) "RTS_Actor"))))) (Math|Float|SelectFloat 1.8e+02 -3e+01 (Utilities|String|Contains (Utilities|String|ToString(Name) (LocalVariables|GetCurrentLandingBoneName)) "_r")))) _returnvalue_2) _returnvalue_2 (Utilities|String|Contains (Utilities|GetObjectName (LocalVariables|GetCurrentAnimation)) "IDLE")))))))